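; BP_Interact is an overlap actor that switches the fox NPC's AI state as actors enter and leave it.
; Both overlap events fetch the BP_NPC_FOX instance via GetActorOfClass and cast its controller to AIC_FOX, without checking which actor overlapped.
; Begin overlap sets the Interact state.
; End overlap sets Leaving, then restores Normal after a short delay.
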(event Collision|EventActorBeginOverlap
  (params (OtherActor :type Actor%20Object%20Reference))
  (bind _returnvalue (Actor|GetActorOfClass "/Game/_Blueprints/_NPC/BP_NPC_FOX.BP_NPC_FOX_C"))
  (bind _asaic_fox (Utilities|Casting|CastToAIC_FOX (AI|GetAIController _returnvalue)))
  (Default|SetStateasInteract _asaic_fox))

(event Collision|EventActorEndOverlap
  (params (OtherActor :type Actor%20Object%20Reference))
  (bind _returnvalue (Actor|GetActorOfClass "/Game/_Blueprints/_NPC/BP_NPC_FOX.BP_NPC_FOX_C"))
  (bind _asaic_fox (Utilities|Casting|CastToAIC_FOX (AI|GetAIController _returnvalue)))
  (Variables|Default|SetAs%20AIC%20FOX _asaic_fox)
  (Default|SetStateasLeaving (Variables|Default|GetAs%20AIC%20FOX))
  (Utilities|FlowControl|Delay 3.0)
  (Default|SetStateasNormal (Variables|Default|GetAs%20AIC%20FOX)))

(fn ConstructionScript)