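; BP_MainPlayer is the player Blueprint that owns the player HUD and plays landing feedback.
; On BeginPlay it creates the WB_PlayerHud widget, stores it and adds it to the viewport.
; The aim-down-sight Enhanced Input action toggles the HUD crosshair on press and release, and landing plays a MetaSound at the actor's location.
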(event Input|EnhancedActionEvents|EnhancedInputActionIA_AimDownSight
  (params (ActionValue :type Boolean) (ElapsedSeconds :type Float%20%28double-precision%29) (TriggeredSeconds :type Float%20%28double-precision%29) (InputAction :type Input%20Action%20Object%20Reference :default "/Game/Input/IA_AimDownSight.IA_AimDownSight"))
  (:Started
    (Default|ToggleCrosshair (Variables|Default|GetMainPlayerHud) true))
  (:Completed
    (Default|ToggleCrosshair (Variables|Default|GetMainPlayerHud) false)))

(event EventBeginPlay
  (bind _returnvalue (UserInterface|CreateWidget "/Game/UI/PlayerHud/WB_PlayerHud.WB_PlayerHud_C"))
  (bind _output_get (Variables|Default|SetMainPlayerHud _returnvalue))
  (UserInterface|Viewport|AddtoViewport _output_get 0))

(event EventOnLanded
  (params (Hit :type Hit%20Result%20Structure%20%28by%20ref%29))
  (Audio|PlaySoundatLocation "/Game/Sounds/Player/Movement/MS_Land.MS_Land" (Transformation|GetActorLocation) "0, 0, 0" 1.0 1.0 0.0 0 0 0 0))

(fn ConstructionScript)