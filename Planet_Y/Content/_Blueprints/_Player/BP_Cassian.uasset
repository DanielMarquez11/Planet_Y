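; Player character Blueprint for Cassian, with HUD, aim crosshair toggle, landing sound, alternating sword slashes and magnetic grapple pull.
; Sword collision overlaps deal damage through the Damageable interface.
; Grapple targeting picks sphere-traced points by camera dot product and line of sight; pulling zeroes gravity and launches toward the point until arrival, jump or dash.
; Tick is empty, leaving grapple detection and movement calls disconnected.
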(event OnComponentBeginOverlap(SwordHitCollision)
  (params (OverlappedComponent :type Primitive%20Component%20Object%20Reference) (OtherActor :type Actor%20Object%20Reference) (OtherComp :type Primitive%20Component%20Object%20Reference) (OtherBodyIndex :type Integer) (bFromSweep :type Boolean) (SweepResult :type Hit%20Result%20Structure%20%28by%20ref%29))
  (if (Utilities|DoesObjectImplementInterface OtherActor "/Script/Planet_Y.Damageable")
    (if (!= OtherActor self)
      (Class|Damageable|TakeDamagetoHealth(Message) OtherActor 1e+02))))

(event Input|EnhancedActionEvents|EnhancedInputActionIA_AimDownSight
  (params (ActionValue :type Boolean) (ElapsedSeconds :type Float%20%28double-precision%29) (TriggeredSeconds :type Float%20%28double-precision%29) (InputAction :type Input%20Action%20Object%20Reference :default "/Game/Input/IA_AimDownSight.IA_AimDownSight"))
  (:Started
    (Default|ToggleCrosshair (Variables|BaseMagnet|GetMainPlayerHud) true))
  (:Completed
    (Default|ToggleCrosshair (Variables|BaseMagnet|GetMainPlayerHud) false)))

(event Input|EnhancedActionEvents|EnhancedInputActionIA_MagneticPull
  (params (ActionValue :type Boolean) (ElapsedSeconds :type Float%20%28double-precision%29) (TriggeredSeconds :type Float%20%28double-precision%29) (InputAction :type Input%20Action%20Object%20Reference :default "/Game/Input/IA_MagneticPull.IA_MagneticPull"))
  (:Started
    (Utilities|IsValid (Variables|BaseMagnet|GetGrapplePointRef)
      (:Is%20Valid
        (if (<= (Math|Vector|VectorLength (- (Transformation|GetActorLocation) (Transformation|GetActorLocation (Variables|BaseMagnet|GetGrapplePointRef)))) (Variables|Default|GetGrappleRange))
          (bind _output_get (Variables|BaseMagnet|SetCurrentGrapplePoint (Variables|BaseMagnet|GetGrapplePointRef)))
          (Variables|BaseMagnet|SetGrappleDestination (Transformation|GetActorLocation _output_get))
          (Transformation|SetActorRotation (Math|Rotator|MakeRotator 0.0 0.0 (.yaw (Math|Rotator|FindLookatRotation (Transformation|GetActorLocation) (Variables|BaseMagnet|GetGrappleDestination)))))
          (Default|Use (Variables|BaseMagnet|GetGrapplePointRef))
          (MagnetMovement|StartGrappleMovement))))))

(event Input|EnhancedActionEvents|EnhancedInputActionIA_Dash
  (params (ActionValue :type Boolean) (ElapsedSeconds :type Float%20%28double-precision%29) (TriggeredSeconds :type Float%20%28double-precision%29) (InputAction :type Input%20Action%20Object%20Reference :default "/Game/Input/IA_Dash.IA_Dash"))
  (if (== (Variables|Default|GetbMovingToGrapplePoint) true)
    (MagnetMovement|StopGrappleMovement)))

(event Input|EnhancedActionEvents|EnhancedInputActionIA_Jump
  (params (ActionValue :type Boolean) (ElapsedSeconds :type Float%20%28double-precision%29) (TriggeredSeconds :type Float%20%28double-precision%29) (InputAction :type Input%20Action%20Object%20Reference :default "/Game/Input/IA_Jump.IA_Jump"))
  (:Started
    (if (== (Variables|Default|GetbMovingToGrapplePoint) true)
      (MagnetMovement|StopGrappleMovement))))

(event Input|EnhancedActionEvents|EnhancedInputActionIA_Shoot
  (params (ActionValue :type Boolean) (ElapsedSeconds :type Float%20%28double-precision%29) (TriggeredSeconds :type Float%20%28double-precision%29) (InputAction :type Input%20Action%20Object%20Reference :default "/Game/Input/IA_Shoot.IA_Shoot"))
  (:Started
    (if (not (Variables|Default|GetbIsSlashing))
      (Variables|Default|SetbIsSlashing true)
      (Utilities|FlowControl|FlipFlop
        (:A
          (Animation|Montage|PlayMontage (Variables|Character|GetMesh) "/Game/Art/_Cassian/Animations/AM_SlashOne.AM_SlashOne"
            (:OnCompleted
              _)
            (:OnInterrupted
              _))
          (Variables|Default|SetbIsSlashing false))
        (:B
          (Animation|Montage|PlayMontage (Variables|Character|GetMesh) "/Game/Art/_Cassian/Animations/AM_SlashTwo.AM_SlashTwo"
            (:OnCompleted
              _)
            (:OnInterrupted
              _))
          (Variables|Default|SetbIsSlashing false))))))

(event EventBeginPlay
  (bind _returnvalue (UserInterface|CreateWidget "/Game/UI/PlayerHud/WB_PlayerHud.WB_PlayerHud_C"))
  (bind _output_get (Variables|BaseMagnet|SetMainPlayerHud _returnvalue))
  (UserInterface|Viewport|AddtoViewport _output_get 0))

(event EventOnLanded
  (params (Hit :type Hit%20Result%20Structure%20%28by%20ref%29))
  (Audio|PlaySoundatLocation "/Game/Sounds/Player/Movement/MS_Land.MS_Land" (Transformation|GetActorLocation) "0, 0, 0" 1.0 1.0 0.0 0 0 0 0))

(event EventTick
  (params (DeltaSeconds :type Float%20%28single-precision%29)))

(fn ConstructionScript)

(fn CheckforGrapplePoints
  (bind _returnvalue (Transformation|GetActorLocation))
  (bind _followcamera (Variables|Default|GetFollowCamera))
  (bind (_outhits _returnvalue_2) (Collision|MultiSphereTraceForObjects _returnvalue _returnvalue (Variables|Default|GetGrappleDetectionRange) (Utilities|Array|MakeArray "ObjectTypeQuery7") false 0 "None"))
  (if _returnvalue_2
    (LocalVariables|SetHighestDotProduct 0.7)
    (bind _array_element (Utilities|Array|ForEachLoopwithBreak _outhits)
      (:LoopBody
        (if (> (Math|Vector|DotProduct (Math|Vector|GetForwardVector _followcamera) (Math|Vector|GetUnitDirection(Vector) (Transformation|GetWorldLocation _followcamera) (Transformation|GetActorLocation (.HitActor (Collision|BreakHitResult _array_element))))) (LocalVariables|GetHighestDotProduct))
          (LocalVariables|SetHighestDotProduct (Math|Vector|DotProduct (Math|Vector|GetForwardVector _followcamera) (Math|Vector|GetUnitDirection(Vector) (Transformation|GetWorldLocation _followcamera) (Transformation|GetActorLocation (.HitActor (Collision|BreakHitResult _array_element))))))
          (Variables|BaseMagnet|SetDetectedActor (.HitActor (Collision|BreakHitResult _array_element)))
          (else
            (BaseMagnetPull|DeactivateGrapplePointRef))))
      (:Completed
        (BaseMagnetPull|ActivateGrapplePoint)))
    (else
      (BaseMagnetPull|DeactivateGrapplePointRef))))

(fn ActivateGrapplePoint
  (Utilities|IsValid (Variables|BaseMagnet|GetDetectedActor)
    (:Is%20Valid
      (bind _outhit (Collision|LineTraceByChannel (Transformation|GetWorldLocation (Variables|Default|GetFollowCamera)) (Transformation|GetActorLocation (Variables|BaseMagnet|GetDetectedActor)) "TraceTypeQuery1" false 0 "None"))
      (if (== (.hitactor _outhit) (Variables|BaseMagnet|GetDetectedActor))
        (if (!= (Variables|BaseMagnet|GetDetectedActor) (Variables|BaseMagnet|GetGrapplePointRef))
          (bind _asbp_grapple_point (Utilities|Casting|CastToBP_GrapplePoint (Variables|BaseMagnet|GetDetectedActor)))
          (BaseMagnetPull|DeactivateGrapplePointRef)
          (bind _output_get (Variables|BaseMagnet|SetGrapplePointRef _asbp_grapple_point))
          (Default|Activate _output_get))
        (else
          (BaseMagnetPull|DeactivateGrapplePointRef))))))

(fn DeactivateGrapplePointRef
  (Utilities|IsValid (Variables|BaseMagnet|GetGrapplePointRef)
    (:Is%20Valid
      (Default|Deactivate (Variables|BaseMagnet|GetGrapplePointRef))
      (Variables|BaseMagnet|SetGrapplePointRef 0))))

(fn GrappleMovement
  (bind _launchdirection (MagnetMovement|GetLaunchDirection))
  (Character|LaunchCharacter (* _launchdirection (Variables|Default|GetMagnetPullForce)) true true)
  (if (< (Math|Vector|Distance(Vector) (Transformation|GetActorLocation) (Variables|BaseMagnet|GetGrappleDestination)) 4e+01)
    (MagnetMovement|StopGrappleMovement)))

(fn StartGrappleMovement
  (Variables|/Script/Engine.CharacterMovementComponent|SetGravityScale (Variables|Character|GetCharacterMovement) 0.0)
  (Components|Movement|StopMovementImmediately (Variables|Character|GetCharacterMovement))
  (Pawn|Components|CharacterMovement|SetMovementMode (Variables|Character|GetCharacterMovement) "MOVE_Falling" 0)
  (Variables|Default|SetbMovingToGrapplePoint true))

(fn StopGrappleMovement
  (Variables|/Script/Engine.CharacterMovementComponent|SetGravityScale (Variables|Character|GetCharacterMovement) 2.5)
  (Variables|Default|SetbMovingToGrapplePoint false))

(fn GetLaunchDirection
  (return (Math|Vector|Normalize (- (Variables|BaseMagnet|GetGrappleDestination) (Transformation|GetActorLocation)))))

(fn EnableHitCollision
  (Collision|SetCollisionEnabled (Variables|Default|GetSwordHitCollision) "QueryOnly"))

(fn DisableHitCollision
  (Collision|SetCollisionEnabled (Variables|Default|GetSwordHitCollision) "NoCollision"))