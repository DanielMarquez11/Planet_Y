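; BP_MeteorCheckpoint is a scripted meteor fall, triggered when the player pawn enters its box.
; BeginPlay hides the meteor at its start point and computes the direction to the end point.
; On overlap it appears with spawn and falling sounds, and Tick moves it at FallSpeed without sweeping.
; When the end-point distance check passes, a DoOnce spawns explosion particles and sound, then hides and stops the meteor.
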(event OnComponentBeginOverlap(Box)
  (params (OverlappedComponent :type Primitive%20Component%20Object%20Reference) (OtherActor :type Actor%20Object%20Reference) (OtherComp :type Primitive%20Component%20Object%20Reference) (OtherBodyIndex :type Integer) (bFromSweep :type Boolean) (SweepResult :type Hit%20Result%20Structure%20%28by%20ref%29))
  (if (== OtherActor (Game|Player|GetPlayerPawn 0))
    (Rendering|SetVisibility (Variables|Default|GetMeteor) true true)
    (Variables|Default|SetbShouldMove true)
    (Audio|PlaySound2D "/Game/Sounds/Meteor/MeteorSpawn.MeteorSpawn" 1.0 1.0 0.0 0 0)
    (bind _returnvalue (Audio|SpawnSoundAttached "/Game/Sounds/Meteor/MeteorFalling.MeteorFalling" (Variables|Default|GetMeteor) "None" "0, 0, 0" "0, 0, 0" "KeepRelativeOffset" true 1.0 1.0 0.0 0 0))
    (Variables|Default|SetFallingMeteorSound _returnvalue)))

(event EventBeginPlay
  (Rendering|SetVisibility (Variables|Default|GetMeteor) false true)
  (Transformation|SetWorldLocation (Variables|Default|GetMeteor) (Transformation|GetWorldLocation (Variables|Default|GetMeteorStartPoint)) false false)
  (Variables|Default|SetFallDirection (Math|Vector|Normalize (- (Transformation|GetWorldLocation (Variables|Default|GetMeteorEndPoint)) (Transformation|GetWorldLocation (Variables|Default|GetMeteorStartPoint))))))

(event EventTick
  (params (DeltaSeconds :type Float%20%28single-precision%29))
  (if (Variables|Default|GetbShouldMove)
    (Transformation|SetWorldLocation (Variables|Default|GetMeteor) (+ (* DeltaSeconds (* (Variables|Default|GetFallDirection) (Variables|Default|GetFallSpeed))) (Transformation|GetWorldLocation (Variables|Default|GetMeteor))) false false)
    (if (Utilities|GetDistancetoEndPoint)
      (Utilities|FlowControl|DoOnce false
        (:Completed
          (Niagara|SpawnSystematLocation (Variables|Default|GetParticles) (Transformation|GetWorldLocation (Variables|Default|GetMeteorEndPoint)))
          (Audio|Components|Audio|Stop (Variables|Default|GetFallingMeteorSound))
          (Audio|SpawnSoundatLocation "/Game/Sounds/Meteor/MeteorExplosion.MeteorExplosion" (Transformation|GetWorldLocation (Variables|Default|GetMeteorEndPoint)) "0, 0, 0" 1.0 1.0 0.0 0 0)
          (Rendering|SetVisibility (Variables|Default|GetMeteor) false true)
          (Variables|Default|SetbShouldMove false))))))

(fn ConstructionScript)