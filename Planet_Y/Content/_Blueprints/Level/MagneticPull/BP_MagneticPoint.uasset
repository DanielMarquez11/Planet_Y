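; BP_MagneticPoint is a grapple target that shows a detection-node widget while activated for the player.
; While active and unused, Tick grows the widget's fill as the player nears and turns it white within GrappleRange.
; Use plays an animation and pauses those updates for a short timer-driven cooldown.
; The player overlapping the Box disables the Sphere's collision until they leave.
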(event OnComponentBeginOverlap(Box)
  (params (OverlappedComponent :type Primitive%20Component%20Object%20Reference) (OtherActor :type Actor%20Object%20Reference) (OtherComp :type Primitive%20Component%20Object%20Reference) (OtherBodyIndex :type Integer) (bFromSweep :type Boolean) (SweepResult :type Hit%20Result%20Structure%20%28by%20ref%29))
  (if (== OtherActor (Variables|Default|GetPlayerRef))
    (Collision|SetCollisionEnabled (Variables|Default|GetSphere) "NoCollision")))

(event OnComponentEndOverlap(Box)
  (params (OverlappedComponent :type Primitive%20Component%20Object%20Reference) (OtherActor :type Actor%20Object%20Reference) (OtherComp :type Primitive%20Component%20Object%20Reference) (OtherBodyIndex :type Integer))
  (if (== OtherActor (Variables|Default|GetPlayerRef))
    (Collision|SetCollisionEnabled (Variables|Default|GetSphere) "QueryAndPhysics")))

(event EventBeginPlay
  (bind _aswbp_detection_node (Utilities|Casting|CastToWBP_DetectionNode (UserInterface|GetUserWidgetObject (Variables|Default|GetWidget))))
  (Variables|Default|SetWidgetRef _aswbp_detection_node)
  (CallFunction|Deactivate))

(event EventTick
  (params (DeltaSeconds :type Float%20%28single-precision%29))
  (if (and (Variables|Default|GetbIsActive) (not (Variables|Default|GetbIsUsed)))
    (CallFunction|CheckDistancefromPlayer)))

(fn ConstructionScript)

(fn Activate
  (params (PlayerRef :type BP%20Cassian%20Object%20Reference))
  (Variables|Default|SetbIsActive true)
  (Widget|SetVisibility (Variables|Default|GetWidgetRef) "Visible")
  (Variables|Default|SetPlayerRef PlayerRef))

(fn Deactivate
  (Variables|Default|SetbIsActive false)
  (Widget|SetVisibility (Variables|Default|GetWidgetRef) "Hidden"))

(fn CheckDistancefromPlayer
  (bind _returnvalue (Transformation|GetActorLocation))
  (bind _playerref (Variables|Default|GetPlayerRef))
  (bind _playerref_2 (Variables|Default|GetPlayerRef))
  (bind _returnvalue_2 (Transformation|GetActorLocation _playerref))
  (bind _grapplerange (Variables|/Game/_Blueprints/_Player/BP_Cassian.BP_Cassian_C|GetGrappleRange _playerref_2))
  (bind _grappledetectionrange (Variables|/Game/_Blueprints/_Player/BP_Cassian.BP_Cassian_C|GetGrappleDetectionRange _playerref_2))
  (bind _returnvalue_3 (- _returnvalue_2 _returnvalue))
  (bind _returnvalue_4 (Math|Vector|VectorLength _returnvalue_3))
  (bind _returnvalue_5 (Math|Float|MapRangeClamped _returnvalue_4 _grapplerange _grappledetectionrange 45.0 2.0))
  (Class|Image|SetDesiredSizeOverride (Variables|/Game/UI/LevelWidgets/MagneticPull/WBP_DetectionNode.WBP_DetectionNode_C|GetFilling (Variables|Default|GetWidgetRef)) (Math|Vector2D|MakeVector2D _returnvalue_5 _returnvalue_5))
  (Appearance|SetColorandOpacity (Variables|/Game/UI/LevelWidgets/MagneticPull/WBP_DetectionNode.WBP_DetectionNode_C|GetFilling (Variables|Default|GetWidgetRef)) (Math|Color|SelectColor "(R=1.000000,G=1.000000,B=1.000000,A=1.000000)" "(R=0.032292,G=0.032292,B=0.032292,A=1.000000)" (== _returnvalue_5 45.0)) :!class /Script/UMG.Image))

(fn Use
  (bind _widgetref (Variables|Default|GetWidgetRef))
  (Variables|Default|SetbIsUsed true)
  (UserInterface|Animation|PlayAnimation _widgetref (Variables|/Game/UI/LevelWidgets/MagneticPull/WBP_DetectionNode.WBP_DetectionNode_C|GetUseDetectionNode _widgetref) 0.0 1 "Forward" 1.0 true)
  (Utilities|Time|SetTimerbyFunctionName 0 "Reactivate" 2.0))

(fn Reactivate
  (Variables|Default|SetbIsUsed false))