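; BP_CrystalsOnLanded is a short-lived crystal actor for the Crystal Boss, apparently left behind on landing, that sinks away and removes itself.
; BeginPlay waits briefly, enables MoveDown, then destroys the actor once LerpTime has elapsed.
; While MoveDown is set, Tick lerps from the current location toward a point below it along local up, so the descent accelerates and depends on frame rate.
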(event EventTick
  (params (DeltaSeconds :type Float%20%28single-precision%29))
  (bind _returnvalue (Transformation|GetActorLocation))
  (if (Variables|Default|GetbMoveDown)
    (bind _output_get (Variables|Default|SetTimer (+ (Variables|Default|GetTimer) (Utilities|Time|GetWorldDeltaSeconds))))
    (Transformation|SetActorLocation (Math|Vector|Lerp(Vector) _returnvalue (+ _returnvalue (* (Transformation|GetActorUpVector) -3e+01)) (/ _output_get (Variables|Default|GetLerpTime))) false false)))

(event EventBeginPlay
  (Utilities|FlowControl|Delay 2.0)
  (Variables|Default|SetbMoveDown true)
  (Utilities|FlowControl|Delay (Variables|Default|GetLerpTime))
  (Actor|DestroyActor))

(fn ConstructionScript)